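; BP_Pressure is a grabbable valve that the player twists by moving the grabber, with no pressure value computed here.
; Grab stores the grabber and its root-local position, aligns GrabPos from the valve's roll, and returns it with a grab pose.
; While held, Tick turns the local Y movement, times Scale, into valve roll and plays a twist sound every frame.
; Ungrab clears the grabber and plays a click.
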(event `self.ReceiveTick`
  (params (DeltaSeconds :type "Float (single-precision)"))
  (bind _grabber (`self.grabber`)
    (:`then`
      (if true
        (bind _returnvalue (`KismetMathLibrary.InverseTransformLocation` (`SceneComponent.K2_GetComponentToWorld` (`self.DefaultSceneRoot`)) (`SceneComponent.K2_GetComponentLocation` _grabber)))
        (bind (_returnvalue_x _returnvalue_y) (`KismetMathLibrary.BreakVector` (- _returnvalue (`self.lastPos`))))
        (`SceneComponent.K2_AddRelativeRotation` (`self.Valve`) (`KismetMathLibrary.MakeRotator` (* _returnvalue_y (`self.scale`))) false false)
        (set `self.lastPos` _returnvalue)
        (`GameplayStatics.PlaySound2D` "/Game/PrototypeOmega/Audio/Interaction/Pressure_Twist.Pressure_Twist" 0.2 1.0 0.0 null null)))
    (:`else`)))

(event `/Game/PrototypeOmega/Blueprints/Interfaces/interactableInterface.ungrab`
  (set `self.grabber` null)
  (`GameplayStatics.PlaySound2D` "/Game/PrototypeOmega/Audio/Interaction/EngineClick.EngineClick" 0.5 1.0 0.0 null null))

(fn `grab`
  (params (Grabber :type "SceneComponent Object Reference"))
  (returns (GrabPose :type "AnimSequence Object Reference") (GrabPoint :type "SceneComponent Object Reference"))
  (bind _grabpos (`self.grabPos`))
  (bind _relativerotation_roll (`KismetMathLibrary.BreakRotator` (`SceneComponent.RelativeRotation` (`self.Valve`))))
  (bind _output_get (set `self.grabber` Grabber))
  (set `self.lastPos` (`KismetMathLibrary.InverseTransformLocation` (`SceneComponent.K2_GetComponentToWorld` (`self.DefaultSceneRoot`)) (`SceneComponent.K2_GetComponentLocation` _output_get)))
  (bind _result (`/Engine/EditorBlueprintResources/StandardMacros.NegateFloat` _relativerotation_roll)
    (:`  `
      (`SceneComponent.K2_SetRelativeRotation` _grabpos (`KismetMathLibrary.MakeRotator` _result) false false)
      (return (`self.interactGrabPose`) _grabpos))))

(fn `UserConstructionScript`)