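; Test actor with a cube that a grabbing actor can turn around its yaw axis by moving.
; Grab stores the grabber and its position in the local space of the PAr component, and Ungrab clears it.
; While a grabber is set, Tick turns the change in its local X position since the last frame, multiplied by Scale, into relative yaw on the cube.
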(event `self.ReceiveTick`
  (params (DeltaSeconds :type "Float (single-precision)"))
  (bind _targetingactor (`self.TargetingActor`)
    (:`then`
      (bind _returnvalue (`KismetMathLibrary.InverseTransformLocation` (`SceneComponent.K2_GetComponentToWorld` (`self.PAr`)) (`SceneComponent.K2_GetComponentLocation` _targetingactor)))
      (bind _returnvalue_x (`KismetMathLibrary.BreakVector` (- _returnvalue (`self.lastPos`))))
      (`SceneComponent.K2_AddRelativeRotation` (`self.Cube`) (`KismetMathLibrary.MakeRotator` 0.0 0.0 (* _returnvalue_x (`self.scale`))) false false)
      (set `self.lastPos` _returnvalue))
    (:`else`)))

(event `/Game/PrototypeOmega/Blueprints/Interfaces/interactableInterface.ungrab`
  (set `self.TargetingActor` null))

(fn `grab`
  (params (Grabber :type "SceneComponent Object Reference"))
  (returns (GrabPose :type "AnimSequence Object Reference") (GrabPoint :type "SceneComponent Object Reference"))
  (bind _output_get (set `self.TargetingActor` Grabber))
  (set `self.lastPos` (`KismetMathLibrary.InverseTransformLocation` (`SceneComponent.K2_GetComponentToWorld` (`self.PAr`)) (`SceneComponent.K2_GetComponentLocation` _output_get)))
  (return null null))

(fn `UserConstructionScript`)