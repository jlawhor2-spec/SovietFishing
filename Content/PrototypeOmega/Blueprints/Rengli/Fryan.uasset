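; Fryan is a child Blueprint that overrides an inherited Jumpscare event to add a light-and-sound lead-in.
; Jumpscare calls the spookyscarysinging event, which makes a point light visible and plays the Dontpeeonthefloor sound.
; It then waits on a ten-second delay before running the parent's Jumpscare logic.
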(event `spookyscarysinging`
  (`SceneComponent.SetVisibility` (`self.PointLight`) true false)
  (`self.PlaySound` "/Game/PrototypeOmega/Audio/Ambience/dont-pee-on-the-floor.dont-pee-on-the-floor"))

(event `self.Jumpscare`
  (`self.spookyscarysinging`)
  (`KismetSystemLibrary.Delay` 10.0)
  (`parent.Jumpscare`))

(fn `UserConstructionScript`
  (`parent.UserConstructionScript`))