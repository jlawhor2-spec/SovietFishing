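; VR lever actor that arms during a timed or triggered event, flashing a light with an alarm sound until the event ends.
; While armed, Tick eases the handle toward the grabbing hand along local X, clamped to its travel, and calls the empty Activate hook once each time it nears full travel.
; EndEvent disarms it and force-releases the VRPawn's hand, letting the handle ease back to rest.
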(event `self.ReceiveTick`
  (params (DeltaSeconds :type "Float (single-precision)"))
  (bind _returnvalue (* DeltaSeconds 5.0))
  (bind _levercontrol (`self.LeverControl`))
  (bind _relativelocation_x (`KismetMathLibrary.BreakVector` (`SceneComponent.RelativeLocation` _levercontrol)))
  (if (`PrimitiveComponent.bGenerateOverlapEvents` (`self.Capsule`))
    (bind _grabber (`self.Grabber`)
      (:`then`
        (bind _returnvalue_x (`KismetMathLibrary.BreakVector` (`KismetMathLibrary.InverseTransformLocation` (`self.GetTransform`) (`SceneComponent.K2_GetComponentLocation` _grabber))))
        (`SceneComponent.K2_SetRelativeLocation` _levercontrol (`KismetMathLibrary.MakeVector` (`KismetMathLibrary.Lerp` _relativelocation_x (`KismetMathLibrary.FClamp` _returnvalue_x 0.0 (`self.moveDistance`)) _returnvalue)) false false)
        (`self.checkIsActive`)
        (if (`self.isActive`)
          (`/Engine/EditorBlueprintResources/StandardMacros.DoOnce` false :!label _label
            (:`Completed`
              (`self.Activate`)))
          (else
            (goto _label :!via `Reset`))))
      (:`else`))
    (else
      (`SceneComponent.K2_SetRelativeLocation` _levercontrol (`KismetMathLibrary.MakeVector` (`KismetMathLibrary.Lerp` _relativelocation_x 0.0 _returnvalue)) false false))))

(event `Activate`)

(event `/Game/PrototypeOmega/Blueprints/Interfaces/interactableInterface.ungrab`
  (set `self.Grabber` null))

(event `/Game/PrototypeOmega/Blueprints/Interfaces/interactableInterface.startEvent`
  (set `PrimitiveComponent.bGenerateOverlapEvents` true (`self.Capsule`))
  (`self.Flash Light`))

(event `/Game/PrototypeOmega/Blueprints/Interfaces/interactableInterface.endEvent`
  (set `PrimitiveComponent.bGenerateOverlapEvents` false (`self.Capsule`))
  (bind _grabber (`self.Grabber`)
    (:`then`
      (bind _asvrpawn (cast `/Game/PrototypeOmega/Blueprints/StolenFromVRTemplate/VRPawn` (`ActorComponent.GetOwner` _grabber)))
      (if (== null (`/Game/PrototypeOmega/Blueprints/StolenFromVRTemplate/VRPawn.leftHandCollision` _asvrpawn))
        (`/Game/PrototypeOmega/Blueprints/StolenFromVRTemplate/VRPawn.Ungrab Left` _asvrpawn)
        (message `/Game/PrototypeOmega/Blueprints/Interfaces/interactableInterface.ungrab` self)
        (else
          (`/Game/PrototypeOmega/Blueprints/StolenFromVRTemplate/VRPawn.Ungrab Right` _asvrpawn))))
    (:`else`)))

(event `Flash Light`
  (bind _pointlight (`self.PointLight`))
  (bind _returnvalue (not (`SceneComponent.bVisible` _pointlight)))
  (if (`PrimitiveComponent.bGenerateOverlapEvents` (`self.Capsule`)) :!label _label_2
    (`KismetSystemLibrary.Delay` 0.5)
    (if _returnvalue
      (`GameplayStatics.PlaySoundAtLocation` "/Game/PrototypeOmega/Audio/Interaction/Alarm.Alarm" (`SceneComponent.K2_GetComponentLocation` _pointlight) (struct) 1.0 1.0 0.0 null null null null))
    (`SceneComponent.SetVisibility` _pointlight _returnvalue false)
    (goto _label_2)
    (else
      (`SceneComponent.SetVisibility` _pointlight false false))))

(fn `checkIsActive`
  (bind _relativelocation_x (`KismetMathLibrary.BreakVector` (`SceneComponent.RelativeLocation` (`self.LeverControl`))))
  (set `self.isActive` (< (- (`self.moveDistance`) _relativelocation_x) (`self.activeDistance`))))

(fn `grab`
  (params (Grabber :type "SceneComponent Object Reference") (isLeft :type Boolean))
  (returns (GrabPose :type "AnimSequence Object Reference") (GrabPoint :type "SceneComponent Object Reference") (GrabOrigin :type "SceneComponent Object Reference"))
  (locals (GrabPointTemp :type "SceneComponent Object Reference"))
  (set `self.Grabber` Grabber)
  (if isLeft
    (set `local.GrabPointTemp` (`self.grabPointLeft`))
    (else
      (set `local.GrabPointTemp` (`self.grabPointRight`))))
  (return (`self.InteractGrabPose`) (`local.GrabPointTemp`) (`self.grabPointOrigin`)))

(fn `UserConstructionScript`)